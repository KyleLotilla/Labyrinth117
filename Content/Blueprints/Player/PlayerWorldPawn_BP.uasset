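; Player pawn Blueprint that adds audio feedback, enemy contact damage and the win trigger to the player.
; The construction script assigns camera, shooter, inventory, equipment and stats components to pawn variables; BeginPlay links combat stats to level stats.
; Delegates play death, firing, pain and footstep sounds, with footsteps rate-limited by a Tick timer.
; Capsule hits on "Enemy" actors damage the player; overlapping "WIN" actors calls the game mode's WinGame.
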(event `self.ReceiveBeginPlay`
  (bind _returnvalue (`self.GetPlayerCombatStats`))
  (bind _returnvalue_2 (`self.GetPlayerLevelStats`))
  (`LevelStats.SetCombatStats` _returnvalue_2 _returnvalue)
  (add `CombatStats.onNoHealthDelegate` _returnvalue (delegate `OnNoHealth`))
  (add `self.onProjectileFiredDelegate` (delegate `ProjectileFired`))
  ;[1 1 1] Add Sound Effect To FootStep and Player Damaged
  (add `self.onMoveDelegate` (delegate `OnPlayerMove`))
  (add `self.onPlayerDamagedDelegate` (delegate `OnPlayerDamaged`)))

(event `OnNoHealth`
  (`GameplayStatics.PlaySound2D` "/Game/Sounds/Player/Player_Dying.Player_Dying" 2.0 1.0 0.0 null null))

(event `OnPlayerDamaged`
  ;[1 1 1] Add Sound Effect To FootStep and Player Damaged
  (`GameplayStatics.PlaySound2D` "/Game/Sounds/Player/Player_Inpain.Player_Inpain" 3.0 1.0 0.0 null null))

(event `ProjectileFired`
  (`GameplayStatics.PlaySound2D` "/Game/Sounds/Fire/Firing.Firing" 0.3 1.0 0.0 null null))

(event `OnPlayerMove`
  ;[1 1 1] Add Sound Effect To FootStep and Player Damaged
  (if (>= (`self.FootstepTick`) (`self.FootstepRate`))
    (set `self.FootstepTick` 0.0)
    (`GameplayStatics.PlaySound2D` "/Game/Sounds/Footsteps/Walking_5.Walking_5" 2.0 1.5 0.0 null null)))

(event `self.ReceiveTick`
  (params (DeltaSeconds :type "Float (single-precision)"))
  (set `self.FootstepTick` (+ (`self.FootstepTick`) DeltaSeconds)))

(event `self.CapsuleComponent.OnComponentHit`
  (params (HitComponent :type "PrimitiveComponent Object Reference") (OtherActor :type "Actor Object Reference") (OtherComp :type "PrimitiveComponent Object Reference") (NormalImpulse :type "Vector Structure") (Hit :type "HitResult Structure (by ref)"))
  (if (`KismetSystemLibrary.IsValid` OtherActor)
    (if (`self.ActorHasTag` OtherActor "Enemy")
      (bind _asenemy (cast `Enemy` OtherActor))
      (bind _returnvalue (`Enemy.GetEnemyDamage` _asenemy))
      (`self.DamagePlayer` _returnvalue))))

(event `self.CapsuleComponent.OnComponentBeginOverlap`
  (params (OverlappedComponent :type "PrimitiveComponent Object Reference") (OtherActor :type "Actor Object Reference") (OtherComp :type "PrimitiveComponent Object Reference") (OtherBodyIndex :type Integer) (bFromSweep :type Boolean) (SweepResult :type "HitResult Structure (by ref)"))
  (if (`self.ActorHasTag` OtherActor "WIN")
    (bind _asworld_game_mode (cast `WorldGameMode` (`GameplayStatics.GetGameMode`)))
    (`WorldGameMode.WinGame` _asworld_game_mode)))

(fn `UserConstructionScript`
  (set `self.playerCamera` (`self.Camera`))
  (set `self.projectileShooter` (`self.ProjectileShooter_BP`))
  (bind _asinventory (cast `Inventory` (`ChildActorComponent.ChildActor` (`self.Inventory`))))
  (set `self.playerInventory` _asinventory)
  (set `self.playerEquipment` (`self.Equipment`))
  (set `self.playerCombatStats` (`self.CombatStats`))
  (set `self.playerLevelStats` (`self.LevelStats_BP`)))